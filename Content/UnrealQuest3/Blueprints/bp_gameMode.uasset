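; Game mode that handles player respawning and delayed level transitions with background music changes.
; It restarts the last logged-in player on login and whenever their pawn is destroyed, rebinding the destroy event on each restart.
; Jump_to_new_Level fades in a new sound cue if it differs from the current one, then opens a level by name after a short timer.
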(event Custom|Jump_to_new_Level
  (params (Level :type World%20Soft%20Object%20Reference) (LevelName :type Name) (Soundcue :type Sound%20Cue%20Object%20Reference))
  (Utilities|FlowControl|Sequence
    (:then_0
      (if (!= Soundcue (Variables|Default|GetCurntBCM))
        (Audio|Components|Audio|Stop (Variables|Default|GetAudio))
        (bind _output_get (Variables|Default|SetCurntBCM Soundcue))
        (Audio|Components|Audio|SetSound (Variables|Default|GetAudio) _output_get)
        (Audio|Components|Audio|FadeIn (Variables|Default|GetAudio) 1.0 1.0 0.0 "Linear" :!class /Script/Engine.AudioComponent)))
    (:then_1
      (Utilities|Time|SetTimerbyEvent (delegate Custom|Open%20Level) 5.0))))

(event Custom|PawnDied
  (params (DestroyedActor :type Actor%20Object%20Reference))
  (Class|GameModeBase|RestartPlayer (Variables|Default|GetController%20Ref)))

(event Custom|Open%20Level
  (Game|OpenLevel(byName) (stale Custom|Jump_to_new_Level LevelName)))

(event EventPostLogin
  (params (NewPlayer :type Player%20Controller%20Object%20Reference))
  (bind _output_get (Variables|Default|SetController%20Ref NewPlayer))
  (Class|GameModeBase|RestartPlayer _output_get))

(event EventOnRestartPlayer
  (params (NewPlayer :type Controller%20Object%20Reference))
  (Game|BindEventtoOnDestroyed (Pawn|GetControlledPawn NewPlayer) (delegate Custom|PawnDied)))

(fn ConstructionScript)